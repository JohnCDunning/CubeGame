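; BP_Weapon is a hitscan weapon that fires a line trace forward from its Nozzle when WeaponShoot is called.
; Tick counts down the fire-rate cooldown, which gates shooting and resets only when the trace hits.
; Hits spawn a Niagara impact effect aligned to the surface normal.
; Only physics-simulating components receive damage and an impulse along the hit-to-nozzle vector, scaled by ImpactForce and distance.
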(event `self.ReceiveTick`
  (params (DeltaSeconds :type "Float (single-precision)"))
  (set `self.CurrentFireRateCooldown` (`KismetMathLibrary.FClamp` (- (`self.CurrentFireRateCooldown`) DeltaSeconds) 0.0 (`self.FireRate`))))

(fn `UserConstructionScript`)

(fn `WeaponShoot`
  (bind _nozzle (`self.Nozzle`))
  (bind _returnvalue (`SceneComponent.K2_GetComponentLocation` _nozzle))
  (`/Engine/EditorBlueprintResources/StandardMacros.CompareFloat` (`self.CurrentFireRateCooldown`)
    (:`==`
      _)
    (:`<`
      _))
  (bind (_outhit _returnvalue_2) (`KismetSystemLibrary.LineTraceSingle` :`Start` _returnvalue :`End` (+ _returnvalue (* (`SceneComponent.GetForwardVector` _nozzle) 10000.0)) :`TraceChannel` "TraceTypeQuery1" :`DrawDebugType` "ForOneFrame"))
  (if _returnvalue_2
    (bind (_bblockinghit _binitialoverlap _time _distance _location _impactpoint _normal _impactnormal _physmat _hitactor _hitcomponent) (`GameplayStatics.BreakHitResult` _outhit))
    (`NiagaraFunctionLibrary.SpawnSystemAtLocation` "/Game/Projects/CubeGame/Blueprints/Particles/NS_Impact.NS_Impact" _location (`KismetMathLibrary.Conv_VectorToRotator` _normal))
    (`|ExecutionSequence`
      (:`then_0`
        (if (`SceneComponent.IsSimulatingPhysics` _hitcomponent "None")
          (`PrimitiveComponent.AddImpulseAtLocation` _hitcomponent (* (- _returnvalue _location) (`self.ImpactForce`)) _location "None")
          (`GameplayStatics.ApplyDamage` _hitactor (`self.Damage`) null null "/Script/Engine.DamageType")))
      (:`then_1`
        (set `self.CurrentFireRateCooldown` (`self.FireRate`))))))