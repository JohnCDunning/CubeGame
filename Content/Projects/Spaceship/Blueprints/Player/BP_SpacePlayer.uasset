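; Player pawn for the Spaceship project that moves on the XY plane and can mount, unmount and operate ship systems.
; Systems report availability through AnnounceSystem, which tracks the last announced one as the mount candidate and draws a debug line to it.
; Debug keys E and Space toggle mounting and fire the mounted system's MainAction.
; Enhanced Input drives swept movement, and Tick stores mouse delta in InputDelta.
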(event Input|EnhancedActionEvents|EnhancedInputActionHorizontalAxis
  (params (ActionValue :type Vector%202D%20Structure) (ElapsedSeconds :type Float%20%28double-precision%29) (TriggeredSeconds :type Float%20%28double-precision%29) (InputAction :type Input%20Action%20Object%20Reference :default "/Game/Input/HorizontalAxis.HorizontalAxis"))
  (bind _returnvalue (Transformation|GetActorLocation))
  (bind _returnvalue_2 (Math|Vector2D|Normalize2D ActionValue))
  (bind _playerspeed (Variables|Default|GetPlayerSpeed))
  (bind _returnvalue_3 (* _playerspeed _returnvalue_2))
  (bind (_x _y) (Math|Vector2D|BreakVector2D _returnvalue_3))
  (:Triggered
    (Transformation|SetActorLocation (Math|Vector|MakeVector (+ _x (.x _returnvalue)) (+ _y (.y _returnvalue)) (.z _returnvalue)) true false)))

(event EventBeginPlay
  (bind _asplayer_controller (Utilities|Casting|CastToPlayerController (Pawn|GetController)))
  (Input|AddMappingContext (PlayerController|LocalPlayerSubsystems|GetEnhancedInputLocalPlayerSubsystem _asplayer_controller) "/Game/Input/Player.Player" 0 "(bIgnoreAllPressedKeysUntilRelease=True,bForceImmediately=False)"))

(event Collision|EventActorBeginOverlap
  (params (OtherActor :type Actor%20Object%20Reference)))

(event EventTick
  (params (DeltaSeconds :type Float%20%28single-precision%29))
  (bind _returnvalue (Game|GetPlayerController 0))
  (bind _lastannouncedsystem (Variables|System|GetLastAnnouncedSystem))
  (bind (_deltax _deltay) (Class|PlayerController|GetInputMouseDelta _returnvalue))
  (Variables|Default|SetInputDelta (Math|Vector2D|MakeVector2D _deltax _deltay))
  (Utilities|IsValid _lastannouncedsystem
    (:Is%20Valid
      (Rendering|Debug|DrawDebugLine (Transformation|GetActorLocation) (Transformation|GetActorLocation _lastannouncedsystem) "(R=1.000000,G=0.107830,B=0.000000,A=1.000000)" 0.0 0.0))))

(event Input|KeyboardEvents|DebugKeySpaceBar
  (params (Key :type Key%20Structure :default "None") (ActionValue :type Input%20Action%20Value%20Structure))
  (bind _mountedsystem (Variables|System|GetMountedSystem))
  (:Pressed
    (Utilities|IsValid _mountedsystem
      (:Is%20Valid
        (Default|MainAction _mountedsystem)))))

(event Input|KeyboardEvents|DebugKeyE
  (params (Key :type Key%20Structure :default "None") (ActionValue :type Input%20Action%20Value%20Structure))
  (bind _self self)
  (bind _lastannouncedsystem (Variables|System|GetLastAnnouncedSystem))
  (:Pressed
    (if (Variables|System|GetHasMountedSystem)
      (Default|UnmountSystem (Variables|System|GetMountedSystem) _self)
      (Variables|System|SetHasMountedSystem false)
      (Variables|System|SetMountedSystem 0)
      (else
        (Utilities|IsValid _lastannouncedsystem
          (:Is%20Valid
            (Variables|System|SetMountedSystem _lastannouncedsystem)
            (Default|MountSystem _lastannouncedsystem _self)
            (Variables|System|SetHasMountedSystem true)))))))

(fn ConstructionScript)

(fn AnnounceSystem
  (params (AnnouncingSystem :type BP%20System%20Object%20Reference) (IsAvailable :type Boolean))
  (if IsAvailable
    (Variables|System|SetLastAnnouncedSystem AnnouncingSystem)
    (elif (== AnnouncingSystem (Variables|System|GetLastAnnouncedSystem))
      (Variables|System|SetLastAnnouncedSystem 0))))