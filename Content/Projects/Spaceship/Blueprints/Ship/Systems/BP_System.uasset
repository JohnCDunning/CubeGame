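; BP_System is a ship system actor that a BP_SpacePlayer can mount, with a placeholder MainAction that only prints "Not Implemented".
; An interaction volume announces the system to overlapping players and tracks them.
; MountSystem withdraws those announcements, snaps the player to MountPosition and matches the unmount point's height to theirs, all inside the announced-players loop.
; UnmountSystem detaches the player and teleports them to UnmountPosition.
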(event `self.Interaction Bounds.OnComponentBeginOverlap`
  (params (OverlappedComponent :type "PrimitiveComponent Object Reference") (OtherActor :type "Actor Object Reference") (OtherComp :type "PrimitiveComponent Object Reference") (OtherBodyIndex :type Integer) (bFromSweep :type Boolean) (SweepResult :type "HitResult Structure (by ref)"))
  (bind _asbp_space_player (cast `/Game/Projects/Spaceship/Blueprints/Player/BP_SpacePlayer` OtherActor))
  (`/Game/Projects/Spaceship/Blueprints/Player/BP_SpacePlayer.AnnounceSystem` _asbp_space_player self true)
  (`BlueprintSetLibrary.Set_Add` (`self.AnnoucedPlayers`) _asbp_space_player))

(event `self.Interaction Bounds.OnComponentEndOverlap`
  (params (OverlappedComponent :type "PrimitiveComponent Object Reference") (OtherActor :type "Actor Object Reference") (OtherComp :type "PrimitiveComponent Object Reference") (OtherBodyIndex :type Integer))
  (bind _asbp_space_player (cast `/Game/Projects/Spaceship/Blueprints/Player/BP_SpacePlayer` OtherActor))
  (`/Game/Projects/Spaceship/Blueprints/Player/BP_SpacePlayer.AnnounceSystem` _asbp_space_player self false)
  (`BlueprintSetLibrary.Set_Remove` (`self.AnnoucedPlayers`) _asbp_space_player))

(fn `MainAction`
  (`KismetSystemLibrary.PrintString` "Not Implemented" true true (struct :`R` 1.0 :`G` 0.034335 :`A` 1.0)))

(fn `MountSystem`
  (params (Player :type "/Game/Projects/Spaceship/Blueprints/Player/BP_SpacePlayer Object Reference"))
  (bind _annoucedplayers (`self.AnnoucedPlayers`))
  (bind _unmountposition (`self.UnmountPosition`))
  (bind (_returnvalue_x _returnvalue_y) (`KismetMathLibrary.BreakVector` (`SceneComponent.K2_GetComponentLocation` _unmountposition)))
  (bind _result (`BlueprintSetLibrary.Set_ToArray` _annoucedplayers))
  (for _array_element _result
    (`/Game/Projects/Spaceship/Blueprints/Player/BP_SpacePlayer.AnnounceSystem` _array_element self false)
    (bind _output_get (set `self.MountedPlayer` Player))
    (bind (_returnvalue_x_2 _returnvalue_y_2 _returnvalue_z) (`KismetMathLibrary.BreakVector` (`self.K2_GetActorLocation` _output_get)))
    (`SceneComponent.K2_SetWorldLocation` _unmountposition (`KismetMathLibrary.MakeVector` _returnvalue_x _returnvalue_y _returnvalue_z) false false)
    (`self.K2_AttachToComponent` _output_get (`self.MountPosition`) "None" "SnapToTarget" "SnapToTarget" "KeepWorld" true))
  (`BlueprintSetLibrary.Set_Clear` _annoucedplayers))

(fn `UnmountSystem`
  (params (Player :type "/Game/Projects/Spaceship/Blueprints/Player/BP_SpacePlayer Object Reference"))
  (bind _unmountposition (`self.UnmountPosition`))
  (`self.K2_DetachFromActor` Player "KeepWorld" "KeepWorld" "KeepWorld")
  (`self.K2_SetActorLocationAndRotation` Player (`SceneComponent.K2_GetComponentLocation` _unmountposition) (`SceneComponent.K2_GetComponentRotation` _unmountposition) true true)
  (set `self.MountedPlayer` null))

(fn `UserConstructionScript`)