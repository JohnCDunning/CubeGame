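; BP_Player is the player actor, which turns toward the mouse cursor, moves via Enhanced Input and fires a weapon.
; Tick traces under the cursor, draws a debug sphere and smoothly turns the actor toward the hit at its own height.
; Holding left mouse, polled directly on Tick, fires the child-actor BP_Weapon cached at BeginPlay.
; The movement action applies a normalized, swept XY location offset without delta-time scaling.
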(event `self.ReceiveTick`
  (params (DeltaSeconds :type "Float (single-precision)"))
  (bind _returnvalue (`self.K2_GetActorLocation`))
  (bind _returnvalue_2 (`GameplayStatics.GetPlayerController` 0))
  (bind (_worldlocation _worlddirection) (`PlayerController.DeprojectMousePositionToWorld` _returnvalue_2))
  ;[1 1 1] Trace from camera to get the look pos
  (`|ExecutionSequence`
    (:`then_0`
      (bind (_outhit _returnvalue_3) (`KismetSystemLibrary.LineTraceSingle` _worldlocation (+ _worldlocation (* _worlddirection 10000.0)) "TraceTypeQuery1"))
      (if _returnvalue_3
        (bind (_bblockinghit _binitialoverlap _time _distance _location) (`GameplayStatics.BreakHitResult` _outhit))
        (`KismetSystemLibrary.DrawDebugSphere` _location 3.0 12 (struct :`R` 0.289754 :`G` 0.950219 :`B` 1.0 :`A` 1.0) 0.0 1.0)
        (bind (_x _y) (`KismetMathLibrary.BreakVector3f` _location))
        ;[1 1 1] Lookat Trace Hit
        (`self.K2_SetActorRotation` (`KismetMathLibrary.RInterpTo` (`self.K2_GetActorRotation`) (`KismetMathLibrary.FindLookAtRotation` _returnvalue (`KismetMathLibrary.MakeVector` _x _y (`.Z` (`KismetMathLibrary.BreakVector3f` _returnvalue)))) (* (`GameplayStatics.GetWorldDeltaSeconds`) (`self.PlayerTurnSpeed`)) 1.0))))
    (:`then_1`
      (if (`PlayerController.IsInputKeyDown` _returnvalue_2 "LeftMouseButton")
        (`/Game/Blueprints/Weapons/BP_Weapon.WeaponShoot` (`self.ActiveWeapon`))))))

(event `self.ReceiveBeginPlay`
  (`|ExecutionSequence`
    (:`then_0`
      (bind _asbp_weapon (cast `/Game/Blueprints/Weapons/BP_Weapon` (`ChildActorComponent.ChildActor` (`self.BP_Weapon`))))
      (set `self.ActiveWeapon` _asbp_weapon))
    (:`then_1`
      (bind _asplayer_controller (cast `PlayerController` (`self.GetController`)))
      (`EnhancedInputSubsystemInterface.AddMappingContext` (pcsubsystem `EnhancedInputLocalPlayerSubsystem` _asplayer_controller) "/Game/Input/Player.Player" 0 (struct)))))

(event `EnhancedInput|/Game/Input/HorizontalAxis`
  (params (ActionValue :type "Vector2D Structure") (ElapsedSeconds :type "Float (double-precision)") (TriggeredSeconds :type "Float (double-precision)") (InputAction :type "InputAction Object Reference" :default "/Game/Input/HorizontalAxis.HorizontalAxis"))
  (bind (_returnvalue_x _returnvalue_y _returnvalue_z) (`KismetMathLibrary.BreakVector` (`self.K2_GetActorLocation`)))
  (bind (_x _y) (`KismetMathLibrary.BreakVector2D` (* (`self.PlayerSpeed`) (`KismetMathLibrary.Normal2D` ActionValue))))
  (:`Triggered`
    (`self.K2_SetActorLocation` (`KismetMathLibrary.MakeVector` (+ _x _returnvalue_x) (+ _y _returnvalue_y) _returnvalue_z) true)))

(fn `Shoot`
  (`/Game/Blueprints/Weapons/BP_Weapon.WeaponShoot` (`self.ActiveWeapon`)))

(fn `UIFunction`
  (params (UI :type "WidgetComponent Object Reference"))
  (`SceneComponent.K2_SetWorldRotation` UI (`KismetMathLibrary.FindLookAtRotation` (`SceneComponent.K2_GetComponentLocation` UI) (`PlayerCameraManager.GetCameraLocation` (`GameplayStatics.GetPlayerCameraManager` 0))) false false))

(fn `UserConstructionScript`)