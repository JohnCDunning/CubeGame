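; BP_EnemySphere is an enemy that moves and attacks by adding physics force to its static mesh.
; MoveAttack pushes along a given direction, scaled by AttackForce as an acceleration change, only when the cooldown has run out, then restarts it.
; Tick counts the cooldown down to zero.
; AnyDamage and a separate ApplyDamage function duplicate the same logic, subtracting from Health and destroying the actor at zero or below.
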(event `self.ReceiveTick`
  (params (DeltaSeconds :type "Float (single-precision)"))
  ;[1 1 1] Tick cooldown
  (set `self.AttackCooldownCurrent` (`KismetMathLibrary.FClamp` (- (`self.AttackCooldownCurrent`) DeltaSeconds) 0.0 (`self.AttackCooldown`))))

(event `self.ReceiveAnyDamage`
  (params (Damage :type "Float (single-precision)") (DamageType :type "DamageType Object Reference") (InstigatedBy :type "Controller Object Reference") (DamageCauser :type "Actor Object Reference"))
  (bind _output_get (set `self.Health` (- (`self.Health`) Damage)))
  (`/Engine/EditorBlueprintResources/StandardMacros.CompareFloat` _output_get
    (:`==`
      _)
    (:`<`
      _))
  (`self.K2_DestroyActor`))

(fn `ApplyDamage`
  (params (damage :type "Float (double-precision)"))
  (bind _output_get (set `self.Health` (- (`self.Health`) damage)))
  (`/Engine/EditorBlueprintResources/StandardMacros.CompareFloat` _output_get
    (:`==`
      _)
    (:`<`
      _))
  (`self.K2_DestroyActor`))

(fn `MoveAttack`
  (params (Direction :type "Vector Structure"))
  ;[1 1 1] Add force towards direction, used as attack/move
  (`/Engine/EditorBlueprintResources/StandardMacros.CompareFloat` (`self.AttackCooldownCurrent`)
    (:`==`
      _)
    (:`<`
      _))
  (`PrimitiveComponent.AddForce` (`self.StaticMesh`) (* Direction (`self.AttackForce`)) "None" true)
  (set `self.AttackCooldownCurrent` (`self.AttackCooldown`)))

(fn `UserConstructionScript`)